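; Receives OSC messages from a remote controller to spawn perp, victim and bystander NPCs and end the simulation.
; Toggle addresses pick the NPC type and tag, and a spawn button calls SpawnChild.
; Each type fills its spawn points in turn (perp and victim lists shuffled) with a short debounce, and perps spawn as AI running BT_Perp.
; The end button spawns an end-sim widget actor, then quits after a delay.
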(event `self.ReceiveBeginPlay`
  ;[1 1 1] Everytime OSC receives an input, Event will fire
  (set `self.bAreCharParametersSet` false)
  (add `OscReceiverComponent.OnOscReceived` (`self.OscReceiver`) (delegate `OSC Received`))
  ;[1 1 1] Create array of spawn points and shuffle array to randomize
  (bind _outactors (`GameplayStatics.GetAllActorsOfClass` "/Game/BrightLineTest1/Core/SpawnPoints/BP_PerpSpawnPoint.BP_PerpSpawnPoint_C"))
  (bind _output_get (set `self.PerpSpawnPointArray` _outactors))
  (`KismetArrayLibrary.Array_Shuffle` _output_get)
  (bind _outactors_2 (`GameplayStatics.GetAllActorsOfClass` "/Game/BrightLineTest1/Core/SpawnPoints/BP_VictimSpawnPoint1.BP_VictimSpawnPoint1_C"))
  (bind _output_get_2 (set `self.VictSpawnPointArray` _outactors_2))
  (`KismetArrayLibrary.Array_Shuffle` _output_get_2)
  (bind _outactors_3 (`GameplayStatics.GetAllActorsOfClass` "/Game/BrightLineTest1/Core/SpawnPoints/BP_BystanderSpawnPoint.BP_BystanderSpawnPoint_C"))
  (set `self.BystandSpawnPointArray` _outactors_3))

(event `OSC Received`
  (params (Address :type "Name (by ref)") (Data :type "Array of OscDataElemStruct Structure (by ref)") (SenderIp :type String))
  (set `self.SpawnAddress` Address)
  (`|ExecutionSequence`
    (:`then_0`
      (switch `string` (`KismetStringLibrary.Conv_NameToString` (`self.SpawnAddress`))
        (:`/Controller1/ToggleSpawnType/1/1`
          (if (stale _bool)
            (set `self.SKMaterial_Ref` "/Game/BrightLineTest1/MaterialLibrary/M_Perp_Body_Inst.M_Perp_Body_Inst")
            (set `self.SpawnNPCType` "/Game/BrightLineTest1/Characters/BP_Perp_Child.BP_Perp_Child_C")
            (set `self.SpawnWeapon` true)
            (set `self.NPCTag` "perp")))
        (:`/Controller1/ToggleSpawnType/2/1`
          (if (stale _bool)
            (set `self.SKMaterial_Ref` "/Game/BrightLineTest1/MaterialLibrary/M_Victim_Body_Inst.M_Victim_Body_Inst")
            (set `self.SpawnNPCType` "/Game/BrightLineTest1/Characters/BP_Victim_Child.BP_Victim_Child_C")
            (set `self.SpawnWeapon` false)
            (set `self.NPCTag` "victim")))
        (:`/Controller1/ToggleSpawnType/3/1`
          (if (stale _bool)
            (set `self.SKMaterial_Ref` "/Game/BrightLineTest1/MaterialLibrary/M_Bystander_Body_Inst1.M_Bystander_Body_Inst1")
            (set `self.SpawnNPCType` "/Game/BrightLineTest1/Characters/BP_Bystander_Child.BP_Bystander_Child_C")
            (set `self.SpawnWeapon` false)
            (set `self.NPCTag` "bystander")))
        (:`/Controller1/Spawn1`
          (`self.SpawnChild` (`self.SpawnNPCType`)))
        (:`/Controller1/Push5`
          (`/Engine/EditorBlueprintResources/StandardMacros.DoOnce` false
            (:`Completed`
              (`self.End sim`))))))
    (:`then_1`
      (bind _bool (`self.SplitOSCData` (`KismetStringLibrary.Conv_NameToString` Address) Data SenderIp)))))

(event `SpawnChild`
  (params (SpawnType :type "Actor Class Reference"))
  (bind _perpspawnpointarray (`self.PerpSpawnPointArray`))
  (bind _victspawnpointarray (`self.VictSpawnPointArray`))
  (bind _bystandspawnpointarray (`self.BystandSpawnPointArray`))
  (bind _bystspawnpointindex (`self.BystSpawnPointIndex`))
  ;[1 1 1] spawn npc logic
  (switch `name` (`self.NPCTag`)
    (:`perp`
      (`/Engine/EditorBlueprintResources/StandardMacros.DoOnce` false :!label _label
        (:`Completed`
          (if (not (== (`self.PerpSpawnPointIndex`) (`KismetArrayLibrary.Array_Length` _perpspawnpointarray)))
            (bind _returnvalue (`AIBlueprintHelperLibrary.SpawnAIFromClass` (`self.PawnClass`) "/Game/BrightLineTest1/Core/AI/BT_Perp.BT_Perp" (.location (`self.GetTransform` (`|GetArrayItem` _perpspawnpointarray (`self.PerpSpawnPointIndex`)))) (.rotation (`self.GetTransform` (`|GetArrayItem` _perpspawnpointarray (`self.PerpSpawnPointIndex`)))) true))
            (set `self.SpawnedPerp` _returnvalue)
            (`/Engine/EditorBlueprintResources/StandardMacros.IncrementInt` (`self.PerpSpawnPointIndex`)
              (:`  `
                (message `/Game/BrightLineTest1/Core/BPI_Attach.SetNPCTags` (`self.SpawnedNPC`) (`self.NPCTag`))
                (`KismetSystemLibrary.Delay` 0.2)
                (goto _label :!via `Reset`)))))))
    (:`victim`
      ;[1 1 1] old spawn npc logic not used
      (`/Engine/EditorBlueprintResources/StandardMacros.DoOnce` false :!label _label_2
        (:`Completed`
          (if (not (== (`self.VictSpawnPointIndex`) (`KismetArrayLibrary.Array_Length` _victspawnpointarray)))
            (bind _returnvalue_2 (`|SpawnActorFromClass` (`self.SpawnNPCType`) (`self.GetTransform` (`|GetArrayItem` _victspawnpointarray (`self.VictSpawnPointIndex`))) "AlwaysSpawn" "OverrideRootScale" null null))
            (set `self.SpawnedNPC` _returnvalue_2)
            (`/Engine/EditorBlueprintResources/StandardMacros.IncrementInt` (`self.VictSpawnPointIndex`)
              (:`  `
                (message `/Game/BrightLineTest1/Core/BPI_Attach.SetNPCTags` (`self.SpawnedNPC`) (`self.NPCTag`))
                (`KismetSystemLibrary.Delay` 0.2)
                (goto _label_2 :!via `Reset`)))))))
    (:`bystander`
      (`/Engine/EditorBlueprintResources/StandardMacros.DoOnce` false :!label _label_3
        (:`Completed`
          (if (not (== (`self.BystSpawnPointIndex`) (`KismetArrayLibrary.Array_Length` _bystandspawnpointarray)))
            (bind _returnvalue_3 (`|SpawnActorFromClass` "/Game/BrightLineTest1/Animation/GenericNPCAnimPack/Animations/BP_BystanderChar.BP_BystanderChar_C" (`self.GetTransform` (`|GetArrayItem` _bystandspawnpointarray _bystspawnpointindex)) "AlwaysSpawn" "OverrideRootScale" null _bystspawnpointindex null))
            (set `self.SpawnedNPC` _returnvalue_3)
            (`/Engine/EditorBlueprintResources/StandardMacros.IncrementInt` (`self.BystSpawnPointIndex`)
              (:`  `
                (message `/Game/BrightLineTest1/Core/BPI_Attach.SetNPCTags` (`self.SpawnedNPC`) (`self.NPCTag`))
                (`KismetSystemLibrary.Delay` 0.2)
                (goto _label_3 :!via `Reset`)))))))))

(event `End sim`
  ;[1 1 1] for custom controller
  (`|SpawnActorFromClass` "/Game/BrightLineTest1/Art/UI/BP_EndSimWidget.BP_EndSimWidget_C" (`KismetMathLibrary.MakeTransform` (480.0 -100.0 250.0)) "Undefined" "OverrideRootScale" null null)
  (`KismetSystemLibrary.Delay` 5.0)
  (`KismetSystemLibrary.QuitGame` null "Quit"))

(fn `PrintOSCData`
  (params (Address :type String) (Data :type "Array of OscDataElemStruct Structure") (SenderIP :type String))
  (returns (Bool :type Boolean) (Float :type "Float (double-precision)") (Integer :type Integer) (String :type Name) (OutputPin :type String))
  ;[1 1 1] Print out all data from OSC
  (for _array_element Data
    (bind _returnvalue (`OscFunctionLibrary.AsBool` _array_element))
    (bind _returnvalue_2 (`OscFunctionLibrary.AsFloat` _array_element))
    (bind _returnvalue_3 (`OscFunctionLibrary.AsInt` _array_element))
    (bind _returnvalue_4 (`OscFunctionLibrary.AsString` _array_element))
    (`KismetSystemLibrary.PrintString` (`KismetStringLibrary.Concat_StrStr` (`KismetStringLibrary.Conv_BoolToString` _returnvalue) " / " (`KismetStringLibrary.Conv_DoubleToString` _returnvalue_2) " / " (`KismetStringLibrary.Conv_IntToString` _returnvalue_3) " / " (`KismetStringLibrary.Conv_NameToString` _returnvalue_4) "   ***   Address: " Address) true true (struct :`G` 0.66 :`B` 1.0 :`A` 1.0) 5.0)
    (return _returnvalue _returnvalue_2 _returnvalue_3 _returnvalue_4 Address)))

(fn `SplitOSCData`
  (params (Address :type String) (Data :type "Array of OscDataElemStruct Structure") (SenderIP :type String))
  (returns (Bool :type Boolean) (Float :type "Float (double-precision)") (Integer :type Integer) (String :type Name) (OutputPin :type String))
  ;[1 1 1] Print out all data from OSC
  (for _array_element Data
    (return (`OscFunctionLibrary.AsBool` _array_element) (`OscFunctionLibrary.AsFloat` _array_element) (`OscFunctionLibrary.AsInt` _array_element) (`OscFunctionLibrary.AsString` _array_element) Address)))

(fn `UserConstructionScript`)