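; Child Blueprint for a victim NPC that uses the SK_MannequinNPC mesh and carries no attached weapon.
; Its construction script runs the parent's, then sets the skeletal mesh and its material.
; On BeginPlay it adds itself to NPCArray after the parent logic, and SetNPCTags writes a given tag into the actor tag array.
; AttachWeapon has an empty body.
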(event `self.ReceiveBeginPlay`
  (`parent.ReceiveBeginPlay`)
  (`KismetArrayLibrary.Array_Add` (`self.NPCArray`) self) ; Adds a refernce to itself in BP_NPC
)

(event `/Game/BrightLineTest1/Core/BPI_Attach.SetNPCTags`
  (params (NPCTag :type Name))
  (`KismetArrayLibrary.Array_Set` (`self.ActorTag`) 0 NPCTag))

(fn `AttachWeapon`
  (params (NPSSkeletalMesh :type "SkeletalMeshComponent Object Reference"))
  (return))

(fn `UserConstructionScript`
  (bind _skeletalmesh (`self.SkeletalMesh`))
  (`parent.UserConstructionScript`)
  (`SkinnedMeshComponent.SetSkinnedAssetAndUpdate` _skeletalmesh "/Game/BrightLineTest1/Animation/MannequinNPC/CharacterNPC/MeshNPC/SK_MannequinNPC.SK_MannequinNPC" true)
  (`PrimitiveComponent.SetMaterial` _skeletalmesh 0 (`self.SKMaterial`)))