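; BP_Perp_Child is a child NPC Blueprint for an armed, optionally usable "perp" character.
; Its construction script sets the skeletal mesh and applies a material.
; On BeginPlay it runs parent logic, adds itself to NPCArray, copies ActorTag to its Tags, then spawns an owned BP_Weapon and attaches it through AttachWeaponMessage.
; SetNPCTags writes into ActorTag, and CanUse returns the BisUsable flag.
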(event `self.ReceiveBeginPlay`
  (`parent.ReceiveBeginPlay`)
  (`KismetArrayLibrary.Array_Add` (`self.NPCArray`) self) ; Adds a refernce to itself in BP_NPC
  (set `self.Tags` (`self.ActorTag`))
  (bind _returnvalue (`|SpawnActorFromClass` "/Game/BrightLineTest1/Weapons/BP_Weapon.BP_Weapon_C" (`self.GetTransform`) "AlwaysSpawn" "OverrideRootScale" self null))
  (bind _output_get (set `self.SpawnedAttachment` _returnvalue))
  (message `/Game/BrightLineTest1/Core/BPI_Attach.AttachWeapon` _output_get (`self.SkeletalMesh`)))

(event `/Game/BrightLineTest1/Core/BPI_Attach.SetNPCTags`
  (params (NPCTag :type Name))
  (`KismetArrayLibrary.Array_Set` (`self.ActorTag`) 0 NPCTag))

(fn `CanUse`
  (params (UsingActor :type "Actor Object Reference"))
  (returns (bisUsable :type Boolean))
  (return (`self.bisUsable`)))

(fn `UserConstructionScript`
  (bind _skeletalmesh (`self.SkeletalMesh`))
  (`parent.UserConstructionScript`)
  (`SkinnedMeshComponent.SetSkinnedAssetAndUpdate` _skeletalmesh null true)
  (`PrimitiveComponent.SetMaterial` _skeletalmesh 0 (`self.SKMaterial`)))